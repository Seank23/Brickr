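; Player controller that creates the menu UI container on BeginPlay, shows the mouse cursor and handles switching between menu screens and the game UI.
; Bound events drive menu changes with timeline-lerped horizontal slides, forward or reversed, swapping visibility between slide-out and slide-in.
; Tick polls the level name and calls the game UI load once when the current level is 02_ModelBuilder.
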(event Custom|LoadMenu
  (params (currentMenu :type User%20Widget%20Object%20Reference) (newMenu :type User%20Widget%20Object%20Reference) (reversed :type Boolean))
  ;[1 1 1] Loads new menu screen passed in w/ slide
  (if reversed
    (|SlideBackwardsReversed currentMenu
      (:Finished
        (Widget|SetVisibility currentMenu "Hidden")
        (Widget|SetVisibility newMenu "Visible")
        (|SlideForwards_Reversed newMenu)))
    (else
      (|SlideForwards currentMenu
        (:Finished
          (Widget|SetVisibility currentMenu "Hidden")
          (Widget|SetVisibility newMenu "Visible")
          (|SlideBackwards newMenu))))))

(event Custom|LoadGameUI_Event
  (bind _returnvalue (UserInterface|CreateWidget "/Game/Blueprints/UI/GameUI/_GameUI._GameUI_C"))
  (bind _output_get (Variables|Default|SetmyGameUI _returnvalue))
  (UserInterface|Viewport|AddtoViewport _output_get 0)
  (Variables|Default|SetbShowMouseCursor true))

(event EventBeginPlay
  (bind _returnvalue (UserInterface|CreateWidget "/Game/Blueprints/UI/MenuUI/_MenuUIContainer._MenuUIContainer_C"))
  (Variables|Default|SetmyMenuUIContainer _returnvalue)
  (UserInterface|Viewport|AddtoViewport _returnvalue 0)
  (Variables|Default|SetbShowMouseCursor true)
  (Default|WidgetReady _returnvalue)
  ;[1 1 1] Loads new menu screen passed in w/ slide
  (EventDispatchers|BindEventtoLoadNewMenu (delegate Custom|LoadMenu))
  (EventDispatchers|BindEventtoLoadGameUI (delegate Custom|LoadGameUI_Event)))

(event EventTick
  (params (DeltaSeconds :type Float%20%28single-precision%29))
  (bind _returnvalue (Game|GetCurrentLevelName true))
  (if (and (Utilities|Enum|Equal(Enum) _returnvalue "02_ModelBuilder") (not (Variables|Default|GetisGameLoaded)))
    (Default|CallLoadGameUI)
    (Variables|Default|SetisGameLoaded true)))

(fn ConstructionScript)