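; Player controller for the menu that creates and shows the UI container widget, enables the mouse cursor and animates switches between menu screens.
; LoadMenu, bound as the load-new-menu handler, slides the current screen, hides it on finish, then reveals and slides the new one, with a Reversed flag selecting direction.
; Four timeline-driven slide helpers lerp widget render translation horizontally using a hard-coded 1920-unit offset.
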(event Custom|LoadMenu
  (params (currentMenu :type User%20Widget%20Object%20Reference) (newMenu :type User%20Widget%20Object%20Reference) (reversed :type Boolean))
  ;[1 1 1] Loads new menu screen passed in w/ slide
  (if reversed
    (|SlideBackwardsReversed currentMenu
      (:Finished
        (Widget|SetVisibility currentMenu "Hidden")
        (Widget|SetVisibility newMenu "Visible")
        (|SlideForwards_Reversed newMenu)))
    (else
      (|SlideForwards currentMenu
        (:Finished
          (Widget|SetVisibility currentMenu "Hidden")
          (Widget|SetVisibility newMenu "Visible")
          (|SlideBackwards newMenu))))))

(event EventBeginPlay
  (bind _returnvalue (UserInterface|CreateWidget "/Game/Blueprints/UI/_UIContainer._UIContainer_C"))
  (Variables|Default|SetmyUIContainer _returnvalue)
  (UserInterface|Viewport|AddtoViewport _returnvalue 0)
  (Variables|Default|SetbShowMouseCursor true)
  (Default|WidgetReady _returnvalue)
  ;[1 1 1] Loads new menu screen passed in w/ slide
  (EventDispatchers|BindEventtoLoadNewMenu (delegate Custom|LoadMenu)))

(fn ConstructionScript)